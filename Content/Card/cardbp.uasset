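; Pickup ID card actor that grants the player a key, stored as a HaveKey flag on the GI game instance.
; A Box trigger enables input on the actor while the player character overlaps it and disables it on exit.
; Pressing Pick Card destroys the card's mesh components, sets HaveKey and prints a collection message.
; BeginPlay resets HaveKey to false.
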(event `self.ReceiveBeginPlay`
  (set `/Game/FirstPersonBP/Blueprints/GI.have_key` false (cast `/Game/FirstPersonBP/Blueprints/GI` (`GameplayStatics.GetGameInstance`) :!pure true)))

(event `self.Box.OnComponentBeginOverlap`
  (params (OverlappedComponent :type "PrimitiveComponent Object Reference") (OtherActor :type "Actor Object Reference") (OtherComp :type "PrimitiveComponent Object Reference") (OtherBodyIndex :type Integer) (bFromSweep :type Boolean) (SweepResult :type "HitResult Structure (by ref)"))
  (if (== OtherActor (`GameplayStatics.GetPlayerCharacter` 0))
    (`self.EnableInput` (`GameplayStatics.GetPlayerController` 0))))

(event `InputAction|Pick Card`
  (params (Key :type "Key Structure"))
  (:`Pressed`
    (`/Engine/EditorBlueprintResources/StandardMacros.IsValid` (`self.umbrella_id_card_03_Rectangle001`)
      (:`Is Valid`
        (`ActorComponent.K2_DestroyComponent` (`self.umbrella_id_card_03_Rectangle001`))
        (`ActorComponent.K2_DestroyComponent` (`self.umbrella_id_card_03_Metal_01`))
        (`ActorComponent.K2_DestroyComponent` (`self.umbrella_id_card_03_Metal_02`))
        (`ActorComponent.K2_DestroyComponent` (`self.umbrella_id_card_03_Strap`))
        (`ActorComponent.K2_DestroyComponent` (`self.umbrella_id_card_03_Metal_03`))
        (set `/Game/FirstPersonBP/Blueprints/GI.have_key` true (cast `/Game/FirstPersonBP/Blueprints/GI` (`GameplayStatics.GetGameInstance`) :!pure true))
        (`KismetSystemLibrary.PrintString` "You have collected the card!")))))

(event `self.Box.OnComponentEndOverlap`
  (params (OverlappedComponent :type "PrimitiveComponent Object Reference") (OtherActor :type "Actor Object Reference") (OtherComp :type "PrimitiveComponent Object Reference") (OtherBodyIndex :type Integer))
  (if (== OtherActor (`GameplayStatics.GetPlayerCharacter` 0))
    (`self.DisableInput` (`GameplayStatics.GetPlayerController` 0))))

(fn `UserConstructionScript`)