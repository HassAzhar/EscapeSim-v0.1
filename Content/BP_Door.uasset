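; BP_Door is a player-operated swinging door with open and close sounds.
; Entering its Box enables input on the door, and the "Open door" action alternates through a FlipFlop, guarded by a DoorClosed flag that is true while open.
; The Openclose timeline plays or reverses to drive DoorMesh yaw, and its updates disable input until the player re-enters the Box.
; The key-card check and overlap-exit input disabling are unconnected.
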(event `self.Box.OnComponentBeginOverlap`
  (params (OverlappedComponent :type "PrimitiveComponent Object Reference") (OtherActor :type "Actor Object Reference") (OtherComp :type "PrimitiveComponent Object Reference") (OtherBodyIndex :type Integer) (bFromSweep :type Boolean) (SweepResult :type "HitResult Structure (by ref)"))
  (if (== OtherActor (`GameplayStatics.GetPlayerCharacter` 0))
    (`self.EnableInput` (`GameplayStatics.GetPlayerController` 0))))

(event `InputAction|Open door`
  (params (Key :type "Key Structure"))
  (:`Pressed`
    (`/Engine/EditorBlueprintResources/StandardMacros.FlipFlop`
      (:`A`
        (if (not (`self.door closed`))
          (set `self.door closed` true)
          (`GameplayStatics.PlaySoundAtLocation` "/Game/door-1-open.door-1-open" (`SceneComponent.K2_GetComponentLocation` (`self.DoorMesh`)) (struct) 1.0 1.0 0.0 null null null)
          (bind (_direction _newtrack_0) (`Timeline|open/close` :!label _label)
            (:`Update`
              (`SceneComponent.K2_SetWorldRotation` (`self.DoorMesh`) (`KismetMathLibrary.MakeRotator` 0.0 0.0 _newtrack_0) false false)
              (`self.DisableInput` (`GameplayStatics.GetPlayerController` 0))))))
      (:`B`
        (if (`self.door closed`)
          (set `self.door closed` false)
          (`GameplayStatics.PlaySoundAtLocation` "/Game/door-1-close.door-1-close" (`SceneComponent.K2_GetComponentLocation` (`self.DoorMesh`)) (struct) 1.0 1.0 0.0 null null null)
          (goto _label :!via `Reverse`))))))

(event `self.Box.OnComponentEndOverlap`
  (params (OverlappedComponent :type "PrimitiveComponent Object Reference") (OtherActor :type "Actor Object Reference") (OtherComp :type "PrimitiveComponent Object Reference") (OtherBodyIndex :type Integer)))

(fn `UserConstructionScript`)